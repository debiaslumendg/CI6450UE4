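; Player controller that turns mouse and keyboard input into pawn movement, jumping and shooting, with the cursor shown.
; While the left button is held, Tick traces under the cursor and writes the 2D hit point as the target of the pawn's KinematicBP and KinematicBP_Arrive components.
; Right click spawns a Projectile at the pawn, launched toward the cursor at its maximum speed.
; SpaceBar flags the pawn's Jump component to start.
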(event `self.ReceiveBeginPlay`)

(event `self.ReceiveTick`
  (params (DeltaSeconds :type "Float (single-precision)"))
  (bind _returnvalue (`GameplayStatics.GetPlayerPawn` 0))
  (bind (_hitresult _returnvalue_2) (`self.GetHitResultUnderCursorForObjects` (`|MakeArray` "ObjectTypeQuery7" :!type "EObjectTypeQuery Enum")))
  (if (`self.LeftMouseButtonHeld`)
    (if _returnvalue_2
      (bind _output_get (set `/Game/Movement/KinematicBP.Target` (`KismetMathLibrary.Conv_VectorToVector2D` (`.Location` (`GameplayStatics.BreakHitResult` _hitresult))) (`self.GetComponentByClass` _returnvalue "/Game/Movement/KinematicBP.KinematicBP_C")))
      (set `/Game/Movement/KinematicBP.Target` _output_get (`self.GetComponentByClass` _returnvalue "/Game/Movement/KinematicBP_Arrive.KinematicBP_Arrive_C")))))

(event `InputAction|SpaceBar`
  (params (Key :type "Key Structure"))
  (bind _returnvalue (`self.GetComponentByClass` (`GameplayStatics.GetPlayerPawn` 0) "/Game/Movement/Jump.Jump_C"))
  (:`Pressed`
    (if (`KismetSystemLibrary.IsValid` _returnvalue)
      (set `/Game/Movement/Jump.StartJump` true _returnvalue))))

(event `Key|LeftMouseButton`
  (params (Key :type "Key Structure"))
  (:`Pressed`
    (set `self.LeftMouseButtonHeld` true))
  (:`Released`
    (set `self.LeftMouseButtonHeld` false)))

(event `InputAction|RightMouseButton`
  (params (Key :type "Key Structure"))
  (bind _returnvalue (`self.K2_GetActorLocation` (`GameplayStatics.GetPlayerPawn` 0)))
  (:`Pressed`
    (bind _returnvalue_2 (`|SpawnActorFromClass` "/Game/Projectiles/Projectile.Projectile_C" (`KismetMathLibrary.MakeTransform` (`KismetMathLibrary.MakeVector` (.x _returnvalue) (.y _returnvalue) (+ (.z _returnvalue) 1.0))) "AlwaysSpawn" "OverrideRootScale" null null))
    (bind _kinematicbp (`/Game/Projectiles/Projectile.KinematicBP` _returnvalue_2))
    (set `/Game/Movement/KinematicBP.Velocity` (* (`KismetMathLibrary.Normal2D` (`KismetMathLibrary.Conv_VectorToVector2D` (- (`.Location` (`GameplayStatics.BreakHitResult` (`self.GetHitResultUnderCursorForObjects` (`|MakeArray` "ObjectTypeQuery7" :!type "EObjectTypeQuery Enum")))) _returnvalue))) (`/Game/Movement/KinematicBP.MaxSpeed` _kinematicbp)) _kinematicbp)))

(fn `UserConstructionScript`
  (set `self.bShowMouseCursor` true))