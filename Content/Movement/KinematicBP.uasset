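; Kinematic movement component that moves and rotates its owning actor in 2D from a steering output.
; Each tick, GetSteering caches the target actor's position but returns no computed steering, apparently a base for child behaviors to override.
; Update integrates linear and angular steering, clamps speed, moves the owner without sweep and faces it along velocity, or zeroes velocity on a Nullify flag.
; A debug label shows the component's name above the owner.
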(event `self.ReceiveBeginPlay`
  (if (not (`self.Enabled`))
    (`self.SetComponentTickEnabled` false)))

(event `self.ReceiveTick`
  (params (DeltaSeconds :type "Float (single-precision)"))
  (bind _newparam (`self.GetSteering`))
  (`self.Update` _newparam DeltaSeconds)
  (`KismetSystemLibrary.DrawDebugString` (`KismetMathLibrary.MakeVector` (.x (`Actor.K2_GetActorLocation` (`self.GetOwner`))) (.y (`Actor.K2_GetActorLocation` (`self.GetOwner`))) (+ (.z (`Actor.K2_GetActorLocation` (`self.GetOwner`))) 100.0)) (`KismetSystemLibrary.GetDisplayName` self) null (struct :`R` 1.0 :`A` 1.0)))

(fn `GetNewOrientation`
  (params (CurrentOrientation :type "Float (double-precision)") (Velocity :type "Vector2D Structure"))
  (returns (NewOrientation :type "Float (double-precision)"))
  (bind (_x _y) (`KismetMathLibrary.BreakVector2D` Velocity))
  (if (> (`KismetMathLibrary.VSize2D` Velocity) 0.0)
    (return (`KismetMathLibrary.DegAtan2` _y _x))
    (else
      (return CurrentOrientation))))

(fn `GetSteering`
  (returns (NewParam :type "/Game/Movement/SteeringOutput Structure"))
  (bind _targetactor (`self.TargetActor`))
  (if (`KismetSystemLibrary.IsValid` _targetactor)
    (set `self.Target` (`KismetMathLibrary.Conv_VectorToVector2D` (`Actor.K2_GetActorLocation` _targetactor))))
  (return))

(fn `Update`
  (params (Steering :type "/Game/Movement/SteeringOutput Structure") (DeltaTime :type "Float (double-precision)"))
  (bind (_linear _angular _nullify) (break `/Game/Movement/SteeringOutput` Steering))
  (bind _returnvalue (`self.GetOwner`))
  (bind _returnvalue_2 (* (`self.Velocity`) DeltaTime))
  (if _nullify
    (set `self.Velocity` (0.0 0.0))
    (return)
    (else
      (bind _output_get (set `self.Velocity` (+ (* _linear DeltaTime) (`self.Velocity`))))
      (if (> (`KismetMathLibrary.VSize2D` _output_get) (`self.MaxSpeed`))
        (set `self.Velocity` (* (`KismetMathLibrary.Normal2D` _output_get) (`self.MaxSpeed`))))
      (set `self.Orientation` (+ (* _angular DeltaTime) (`self.Orientation`)))
      (`Actor.K2_SetActorLocation` _returnvalue (+ (`Actor.K2_GetActorLocation` _returnvalue) (`KismetMathLibrary.Conv_Vector2DToVector` _returnvalue_2)) false false)
      (bind _neworientation (`self.GetNewOrientation` (+ (.yaw (`Actor.K2_GetActorRotation` _returnvalue)) (`self.Orientation`)) _returnvalue_2))
      (`Actor.K2_SetActorRotation` _returnvalue (`KismetMathLibrary.MakeRotator` 0.0 0.0 _neworientation) false))))